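; Enemy pawn in the damage system that moves toward a control point, fires projectiles and ragdolls on death.
; On BeginPlay it builds a health bar widget bound to itself.
; Shoot, gated by the damage component's death state, spawns an owned projectile the capsule ignores and binds its impact event to send fixed damage through a TakeDamage message.
; ChasePoint drives AI movement, while DamageResponse is left empty.
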(event Custom|Chase%20Point
  (AI|AIMoveTo self "0, 0, 0" (Variables|Default|GetControlPointRef) 5e+02 false))

(event Custom|CreateWidget
  (bind _returnvalue (UserInterface|CreateWidget "/Game/DamageSystem/Player/HealthBar.HealthBar_C" 0 self))
  (UserInterface|SetWidget (Variables|Default|GetWidget) _returnvalue))

(event Custom|Shoot
  (if (not (Variables|/Game/DamageSystem/BPC_DamageSystem.BPC_DamageSystem_C|GetIsDead (Variables|Default|GetBPC_DamageSystem)))
    (bind _returnvalue (Game|SpawnActorfromClass (Variables|Default|GetProjectileType) (Transformation|GetWorldTransform (Variables|Default|GetScene)) "Undefined" "MultiplyWithRoot" self 0))
    (EventDispatchers|BindEventtoOnProjectileImpact _returnvalue (delegate Custom|DamageEnemu))
    (Collision|IgnoreActorwhenMoving (Variables|Default|GetCapsuleComponent) _returnvalue true)))

(event Custom|DamageEnemu
  (params (Other%20Actor :type Actor%20Object%20Reference) (Hit :type Hit%20Result%20Structure))
  (Class|InterDamageSystem|TakeDamage(Message) Other%20Actor (Utilities|Struct|MakeS_DamageInfo 1e+01 "NewEnumerator1" false "NewEnumerator1")))

(event Collision|EventActorBeginOverlap
  (params (OtherActor :type Actor%20Object%20Reference)))

(event EventTick
  (params (DeltaSeconds :type Float%20%28single-precision%29)))

(event EventBeginPlay
  (CallFunction|CreateWidget))

(event EventPomYouAreDead
  (bind _mesh (Variables|Character|GetMesh))
  (Physics|SetSimulatePhysics _mesh true)
  (Collision|SetCollisionEnabled _mesh "QueryAndPhysics"))

(event EventDamageResponse
  (params (DamageResponse :type DamageResponse%20Enum :default "NewEnumerator0")))

(fn ConstructionScript
  (|CallParentFunction))