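; Player character in the damage system that fires projectiles, shows a health bar and can pause the game.
; Left click spawns BP_ProjectileBase and binds its impact event to send damage info to the hit actor.
; BeginPlay puts a HealthBar in the widget component without calling the parent; death enables mesh physics and disables input.
; GlobalPause and P each toggle the pause menu, game pause and cursor through separate, duplicated FlipFlops.
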(event Custom|DamageEnemy
  (params (Other%20Actor :type Actor%20Object%20Reference) (Hit :type Hit%20Result%20Structure))
  ;[0.3148 0.2042 1] Ataque
  (Class|InterDamageSystem|TakeDamage(Message) Other%20Actor (Utilities|Struct|MakeS_DamageInfo 1e+01 "NewEnumerator1" false "NewEnumerator1")))

(event Collision|EventActorBeginOverlap
  (params (OtherActor :type Actor%20Object%20Reference)))

(event EventTick
  (params (DeltaSeconds :type Float%20%28single-precision%29)))

(event EventBeginPlay
  (bind _returnvalue (UserInterface|CreateWidget "/Game/DamageSystem/Player/HealthBar.HealthBar_C" 0 self))
  (UserInterface|SetWidget (Variables|Default|GetWidget) _returnvalue))

(event EventPomYouAreDead
  (bind _mesh (Variables|Character|GetMesh))
  (Physics|SetSimulatePhysics _mesh true)
  (Collision|SetCollisionEnabled _mesh "QueryAndPhysics")
  (Input|DisableInput (Game|GetPlayerController 0)))

(event EventDamageResponse
  (params (DamageResponse :type DamageResponse%20Enum :default "NewEnumerator0")))

(event Input|MouseEvents|LeftMouseButton
  (params (Key :type Key%20Structure :default "None"))
  ;[0.3148 0.2042 1] Ataque
  (:Pressed
    (bind _returnvalue (Game|SpawnActorfromClass "/Game/DamageSystem/Projectile/BP_ProjectileBase.BP_ProjectileBase_C" (Transformation|GetWorldTransform (Variables|Default|GetScene)) "Undefined" "MultiplyWithRoot" self 0))
    (EventDispatchers|BindEventtoOnProjectileImpact _returnvalue (delegate Custom|DamageEnemy))
    (Collision|IgnoreActorwhenMoving (Variables|Default|GetCapsuleComponent) _returnvalue true)))

(event Input|KeyboardEvents|GlobalPause
  (params (Key :type Key%20Structure :default "None"))
  (bind _returnvalue (Game|GetPlayerController 0))
  ;[1 0.901 0.3785] Menu de Pausa
  (:Pressed
    (Utilities|FlowControl|FlipFlop
      (:A
        (bind _returnvalue_2 (UserInterface|CreateWidget "/Game/Levels/MenuPause/BP_MenuPause.BP_MenuPause_C"))
        (UserInterface|Viewport|AddtoViewport _returnvalue_2 0)
        (Game|SetGamePaused true)
        (Variables|/Script/Engine.PlayerController|SetbShowMouseCursor _returnvalue true))
      (:B
        (Widget|RemovefromParent _returnvalue_2)
        (Game|SetGamePaused false)
        (Variables|/Script/Engine.PlayerController|SetbShowMouseCursor _returnvalue false)))))

(event Input|KeyboardEvents|P
  (params (Key :type Key%20Structure :default "None"))
  (bind _returnvalue (Game|GetPlayerController 0))
  ;[1 0.901 0.3785] Menu de Pausa
  (:Pressed
    (Utilities|FlowControl|FlipFlop
      (:A
        (bind _returnvalue_2 (UserInterface|CreateWidget "/Game/Levels/MenuPause/BP_MenuPause.BP_MenuPause_C"))
        (UserInterface|Viewport|AddtoViewport _returnvalue_2 0)
        (Game|SetGamePaused true)
        (Variables|/Script/Engine.PlayerController|SetbShowMouseCursor _returnvalue true))
      (:B
        (Widget|RemovefromParent _returnvalue_2)
        (Game|SetGamePaused false)
        (Variables|/Script/Engine.PlayerController|SetbShowMouseCursor _returnvalue false)))))

(fn ConstructionScript
  (|CallParentFunction))