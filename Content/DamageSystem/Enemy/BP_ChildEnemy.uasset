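; BP_ChildEnemy is a child enemy Blueprint that automatically fires projectiles on a looping timer started at BeginPlay.
; Each shot spawns the configured projectile class at a scene component's transform, with the enemy as owner and ignored by its moving capsule.
; The projectile's impact event calls back into the enemy, which sends fixed damage info to the hit actor through a TakeDamage interface message.
; A debug event prints damage responses, while disconnected nodes hold unused ragdoll physics setup.
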(event Custom|CustomEvent)

(event Custom|CustomEvent_1
  (params (DamageResponse :type DamageResponse%20Enum :default "NewEnumerator0"))
  (Development|PrintString (Utilities|String|EnumtoString DamageResponse)))

(event Custom|Shoot
  (bind _returnvalue (Game|SpawnActorfromClass (Variables|Default|GetProjectileType) (Transformation|GetWorldTransform (Variables|Default|GetScene)) "Undefined" "MultiplyWithRoot" self 0))
  (EventDispatchers|BindEventtoOnProjectileImpact _returnvalue (delegate Custom|DamageEnemu))
  (Collision|IgnoreActorwhenMoving (Variables|Default|GetCapsuleComponent) _returnvalue true))

(event Custom|DamageEnemu
  (params (Other%20Actor :type Actor%20Object%20Reference) (Hit :type Hit%20Result%20Structure))
  (Class|InterDamageSystem|TakeDamage(Message) Other%20Actor (Utilities|Struct|MakeS_DamageInfo 1e+01 "NewEnumerator1" false "NewEnumerator1")))

(event EventBeginPlay
  (Utilities|Time|SetTimerbyEvent (delegate Custom|Shoot) (Variables|Default|GetShootFrecuency) true))

(event Collision|EventActorBeginOverlap
  (params (OtherActor :type Actor%20Object%20Reference)))

(event EventTick
  (params (DeltaSeconds :type Float%20%28single-precision%29)))

(fn ConstructionScript
  (|CallParentFunction))