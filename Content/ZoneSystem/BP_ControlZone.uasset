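; Capture-point actor where Soldiers and Robots compete over a shared progress value that starts midway.
; Box overlaps count BP_Player pawns per faction using IsHuman.
; Tick steps progress toward the uncontested faction, throttled by a Delay, and holds it when empty or disputed.
; Wins at either limit and all status are only debug prints; the UI widget code is unconnected.
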(event OnComponentBeginOverlap(Box)
  (params (OverlappedComponent :type Primitive%20Component%20Object%20Reference) (OtherActor :type Actor%20Object%20Reference) (OtherComp :type Primitive%20Component%20Object%20Reference) (OtherBodyIndex :type Integer) (bFromSweep :type Boolean) (SweepResult :type Hit%20Result%20Structure%20%28by%20ref%29))
  ;[1 1 1] Increment Counts
  (Utilities|FlowControl|Sequence
    (:then_1
      (bind _asbp_player (Utilities|Casting|CastToBP_Player OtherActor))
      (if (Variables|/Game/DamageSystem/Player/BP_Player.BP_Player_C|GetIsHuman _asbp_player)
        (Utilities|FlowControl|Sequence
          (:then_0
            (Development|PrintString "Es un Soldier"))
          (:then_1
            (Math|Integer|IncrementInt (Variables|Default|GetsoldierCount))))
        (else
          (Utilities|FlowControl|Sequence
            (:then_0
              (Development|PrintString "Es un Robot"))
            (:then_1
              (Math|Integer|IncrementInt (Variables|Default|GetrobotCount)))))))))

(event OnComponentEndOverlap(Box)
  (params (OverlappedComponent :type Primitive%20Component%20Object%20Reference) (OtherActor :type Actor%20Object%20Reference) (OtherComp :type Primitive%20Component%20Object%20Reference) (OtherBodyIndex :type Integer))
  ;[1 1 1] Decrement Counts
  (Utilities|FlowControl|Sequence
    (:then_0
      (bind _asbp_player (Utilities|Casting|CastToBP_Player OtherActor))
      (if (Variables|/Game/DamageSystem/Player/BP_Player.BP_Player_C|GetIsHuman _asbp_player)
        (Math|Integer|DecrementInt (Variables|Default|GetsoldierCount))
        (else
          (Math|Integer|DecrementInt (Variables|Default|GetrobotCount)))))))

(event Custom|CheckControlZone
  ;[1 1 1] Event ControlZone Este evento notifica cuando la zona de control esta en disputa o cunado aumenta a alguna faccion
  (if (and (== (Variables|Default|GetsoldierCount) 0) (== (Variables|Default|GetrobotCount) 0))
    (Development|PrintString "Progreso estable" true true "(R=0.000000,G=0.660000,B=1.000000,A=1.000000)" 0.0)
    (elif (and (> (Variables|Default|GetsoldierCount) 0) (== (Variables|Default|GetrobotCount) 0))
      (Development|PrintString "Aumento progreso Soldiers" true true "(R=0.000000,G=0.660000,B=1.000000,A=1.000000)" 0.0)
      (Utilities|FlowControl|Delay 2.0)
      (Variables|Default|SetzoneCount (Math|Float|Clamp(Float) (+ (Variables|Default|GetzoneCount) 0.1)))
      (elif (and (> (Variables|Default|GetrobotCount) 0) (== (Variables|Default|GetsoldierCount) 0))
        (Development|PrintString "Decremento  progreso Robots" true true "(R=0.000000,G=0.660000,B=1.000000,A=1.000000)" 0.0)
        (Utilities|FlowControl|Delay 2.0)
        (Variables|Default|SetzoneCount (Math|Float|Clamp(Float) (- (Variables|Default|GetzoneCount) 0.1)))
        (elif (and (> (Variables|Default|GetsoldierCount) 0) (> (Variables|Default|GetrobotCount) 0))
          (Development|PrintString "En disputa el punto" true true "(R=0.000000,G=0.660000,B=1.000000,A=1.000000)" 0.0))))))

(event Custom|FactionWinner
  ;[1 1 1] Event FactionWinner
  (if (>= (Variables|Default|GetzoneCount) 1.0)
    (Development|PrintString "Soldiers Winner" true true "(R=0.996078,G=1.000000,B=0.000000,A=1.000000)" 0.0)
    (elif (<= (Variables|Default|GetzoneCount) 0.0)
      (Development|PrintString "Robots Winner" true true "(R=0.996078,G=1.000000,B=0.000000,A=1.000000)" 0.0))))

(event EventBeginPlay
  ;[1 1 1] Start Values
  (Utilities|FlowControl|Sequence
    (:then_1
      (Variables|Default|SetrobotCount 0))
    (:then_2
      (Variables|Default|SetzoneCount 0.5))
    (:then_3
      (Variables|Default|SetsoldierCount 0))))

(event Collision|EventActorBeginOverlap
  (params (OtherActor :type Actor%20Object%20Reference)))

(event EventTick
  (params (DeltaSeconds :type Float%20%28single-precision%29))
  ;[1 1 1] Debugs Counts
  (Utilities|FlowControl|Sequence
    (:then_0
      (Development|PrintString (Utilities|String|ToString(Float) (Variables|Default|GetzoneCount)) true true "(R=0.000000,G=0.660000,B=1.000000,A=1.000000)" 0.0)
      (CallFunction|FactionWinner))
    (:then_1
      (CallFunction|CheckControlZone)
      (Development|PrintString (Utilities|String|ToString(Text) (Utilities|Text|FormatText "Soldiers: {SoldierCount} | Robots: {RobotCount} 
" (Variables|Default|GetsoldierCount) (Variables|Default|GetrobotCount))) true true "(R=1.000000,G=0.000000,B=0.755218,A=1.000000)" 0.0))))

(fn ConstructionScript)